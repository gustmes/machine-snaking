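; Player controller that sets up the game's view through a BP_Camera actor placed in the level.
; On BeginPlay it finds that camera, makes it the view target and reads Width and Height from BP_GameMode.
; It centers the camera at half those dimensions, keeping its Z, and scales the orthographic width to twice the larger one so the view follows the configured size.
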(event `self.ReceiveBeginPlay`
  (bind _returnvalue (`GameplayStatics.GetActorOfClass` "/Game/Blueprints/BP_Camera.BP_Camera_C"))
  (`/Engine/EditorBlueprintResources/StandardMacros.IsValid` _returnvalue
    (:`Is Valid`
      (`self.SetViewTargetWithBlend` _returnvalue)
      (bind _asbp_game_mode (cast `/Game/Blueprints/BP_GameMode` (`GameplayStatics.GetGameMode`)))
      (bind _returnvalue_2 (`KismetMathLibrary.Conv_IntToDouble` (`MachineSnakingGameModeBase.Width` _asbp_game_mode)))
      (bind _returnvalue_3 (`KismetMathLibrary.Conv_IntToDouble` (`MachineSnakingGameModeBase.Height` _asbp_game_mode)))
      (bind (_returnvalue_x _returnvalue_y _returnvalue_z) (`KismetMathLibrary.BreakVector` (`self.K2_GetActorLocation` _returnvalue)))
      (`self.K2_SetActorLocation` _returnvalue (`KismetMathLibrary.MakeVector` (/ _returnvalue_2 2.0) (/ _returnvalue_3 2.0) _returnvalue_z) false false)
      (`CameraComponent.SetOrthoWidth` (`CameraActor.CameraComponent` _returnvalue) (* (`KismetMathLibrary.FMax` _returnvalue_2 _returnvalue_3) 2.0)))))

(fn `UserConstructionScript`)